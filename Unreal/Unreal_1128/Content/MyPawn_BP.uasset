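; MyPawn_BP is a simple pawn that moves in the world XY plane and grows or shrinks its static mesh.
; MoveX and MoveY offset the root by a fixed, frame-rate-dependent step without sweep, only at full axis input in either direction.
; Tick scales the mesh up over time while Grow is held and down otherwise, clamping the scale vector's length.
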(event EventTick
  (params (DeltaSeconds :type Float%20%28single-precision%29))
  (bind _staticmesh (Variables|Default|GetStaticMesh))
  (bind _staticmesh_2 (Variables|Default|GetStaticMesh))
  (bind _returnvalue (Transformation|GetWorldScale _staticmesh_2))
  (if (Variables|Default|GetGrow)
    (Transformation|SetWorldScale3D _staticmesh (Math|Vector|ClampVectorSize (+ _returnvalue DeltaSeconds) 2.0 4.0))
    (else
      (Transformation|SetWorldScale3D _staticmesh (Math|Vector|ClampVectorSize (- _returnvalue DeltaSeconds) 2.0 4.0)))))

(event Input|ActionEvents|InputActionGrow
  (params (Key :type Key%20Structure :default "None"))
  (:Pressed
    (Variables|Default|SetGrow true))
  (:Released
    (Variables|Default|SetGrow false)))

(event Input|AxisEvents|InputAxisMoveX
  (params (AxisValue :type Float%20%28single-precision%29))
  (if (== AxisValue 1.0)
    (Transformation|SetWorldLocation (Variables|Default|GetDefaultSceneRoot) (+ (Transformation|GetWorldLocation (Variables|Default|GetDefaultSceneRoot)) (Math|Vector|MakeVector (* AxisValue 1.0) 0.0 0.0)) false false :!label _label)
    (elif (== AxisValue -1.0)
      (goto _label))))

(event Input|AxisEvents|InputAxisMoveY
  (params (AxisValue :type Float%20%28single-precision%29))
  (if (== AxisValue 1.0)
    (Transformation|SetWorldLocation (Variables|Default|GetDefaultSceneRoot) (+ (Transformation|GetWorldLocation (Variables|Default|GetDefaultSceneRoot)) (Math|Vector|MakeVector 0.0 (* AxisValue 1.0) 0.0)) false false :!label _label)
    (elif (== AxisValue -1.0)
      (goto _label))))

(fn ConstructionScript)